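; LittleMonster1_BP is the Blueprint for a little monster character, and its only logic sets up body-part components.
; The construction script runs the parent's, then attaches the head, left, right, joint, waist (Yao) and tail components to matching Mesh sockets.
; Each attachment snaps location to its socket while keeping world rotation and scale.
; The event graph holds only disabled placeholder events, so any behavior lives outside these graphs.
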(fn `UserConstructionScript`
  (bind _mesh (`self.Mesh`))
  (`parent.UserConstructionScript`)
  (`SceneComponent.K2_AttachToComponent` (`self.Head`) _mesh "Head" "SnapToTarget" "KeepWorld" "KeepWorld" true)
  (`SceneComponent.K2_AttachToComponent` (`self.L`) _mesh "L" "SnapToTarget" "KeepWorld" "KeepWorld" true)
  (`SceneComponent.K2_AttachToComponent` (`self.L_J`) _mesh "L_Joint" "SnapToTarget" "KeepWorld" "KeepWorld" true)
  (`SceneComponent.K2_AttachToComponent` (`self.R`) _mesh "R" "SnapToTarget" "KeepWorld" "KeepWorld" true)
  (`SceneComponent.K2_AttachToComponent` (`self.R_J`) _mesh "R_Joint" "SnapToTarget" "KeepWorld" "KeepWorld" true)
  (`SceneComponent.K2_AttachToComponent` (`self.Yao`) _mesh "Yao" "SnapToTarget" "KeepWorld" "KeepWorld" true)
  (`SceneComponent.K2_AttachToComponent` (`self.Tail`) _mesh "Tail" "SnapToTarget" "KeepWorld" "KeepWorld" true))